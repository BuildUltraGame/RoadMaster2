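; BP_GameRoomGameMode is the game mode for the game room, keeping the room's player roster current as players join.
; On each PostLogin it rebuilds PlayerInformationList from the player controllers, recording each player's name and index and flagging the first as owner.
; It then passes the list and current map ID to RepRoomInformation to share the room state.
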(event `self.K2_PostLogin`
  (params (NewPlayer :type "PlayerController Object Reference"))
  (bind _playerinformationlist (`self.PlayerInformationList`))
  (bind _returnvalue (`self.GetPlayerControllerList`))
  (`KismetArrayLibrary.Array_Clear` _playerinformationlist)
  (for (_array_element _array_index) _returnvalue
    (`KismetArrayLibrary.Array_Add` _playerinformationlist (make `PlayerConnectInformation` (`KismetStringLibrary.Conv_StringToName` (`AdvancedSessionsLibrary.GetPlayerName` _array_element)) 0 (== _array_index 0) _array_index)))
  (`self.RepRoomInformation` (`self.PlayerInformationList`) (`self.CurrentMapID`)))

(fn `UserConstructionScript`)