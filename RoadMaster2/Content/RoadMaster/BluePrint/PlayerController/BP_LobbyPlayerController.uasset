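; Lobby player controller that opens the game-entry UI and manages a shared busy box.
; On BeginPlay, only in standalone net mode, it adds the EnterGameUI widget to the viewport and shows a hand mouse cursor.
; Show and hide functions create a BusyUI widget with caller-supplied text on a raised Z-order and remove it, using a flag to prevent duplicate boxes.
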(event `self.ReceiveBeginPlay`
  (if (`KismetSystemLibrary.IsStandalone`)
    (bind _returnvalue (`|CreateWidget` "/Game/RoadMaster/BluePrint/UI/LobbyUI/EnterGameUI.EnterGameUI_C" (`GameplayStatics.GetPlayerController` 0)))
    (`UserWidget.AddToViewport` _returnvalue 0)
    (set `self.CurrentMouseCursor` "Hand")
    (set `self.bShowMouseCursor` true)))

(fn `BP_HideCommonBusyBox`
  (if (`self.IsBusyBoxShowing`)
    (`Widget.RemoveFromParent` (`self.BusyUI`))
    (set `self.IsBusyBoxShowing` false)))

(fn `BP_ShowCommonBusyBox`
  (params (Text :type String))
  (if (not (`self.IsBusyBoxShowing`))
    (bind _returnvalue (`|CreateWidget` "/Game/RoadMaster/BluePrint/UI/LobbyUI/BusyUI.BusyUI_C" self))
    (`/Game/RoadMaster/BluePrint/UI/LobbyUI/BusyUI.ShowBusyBox` _returnvalue (`KismetTextLibrary.Conv_StringToText` Text))
    (set `self.BusyUI` _returnvalue)
    (`UserWidget.AddToViewport` _returnvalue 5)
    (set `self.IsBusyBoxShowing` true)))

(fn `UserConstructionScript`)