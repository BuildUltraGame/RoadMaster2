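; BP_BaseTrack is a landform track Blueprint that lays a mesh along an editable spline.
; Its Construction Script adds one SplineMeshComponent per pair of neighboring spline points, attached to the spline.
; Each segment uses the StaticMesh and ForwardAxis variables and takes local-space positions and tangents from its two points, so the mesh bends with the curve.
; The Event Graph holds only disabled placeholder events.
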(fn `UserConstructionScript`
  (bind _splinecomponent (`self.SplineComponent`))
  ;[1 1 1 1 60] 根据节点动态赋予spline并且实现每一段材质的角度变更
  (for _index (range 1 (`SplineComponent.GetNumberOfSplinePoints` (`self.SplineComponent`)))
    (bind _returnvalue (`AddComponent|NODE_AddSplineMeshComponent-0`))
    (`StaticMeshComponent.SetStaticMesh` _returnvalue (`self.StaticMesh`))
    (`SplineMeshComponent.SetForwardAxis` _returnvalue (`self.ForwardAxis`) true)
    (`SceneComponent.K2_AttachToComponent` _returnvalue (`self.SplineComponent`) "None" "KeepRelative" "KeepRelative" "KeepRelative" true)
    (bind _returnvalue_2 (- _index 1))
    (`SplineMeshComponent.SetStartAndEnd` _returnvalue (`SplineComponent.GetLocationAtSplinePoint` _splinecomponent _returnvalue_2 "Local") (`SplineComponent.GetTangentAtSplinePoint` _splinecomponent _returnvalue_2 "Local") (`SplineComponent.GetLocationAtSplinePoint` _splinecomponent _index "Local") (`SplineComponent.GetTangentAtSplinePoint` _splinecomponent _index "Local") true)))